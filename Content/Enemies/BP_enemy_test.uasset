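; BP_enemy_test is a test enemy actor that patrols back and forth along the world X axis and can be destroyed through health changes.
; Tick moves it by Speed, SpeedModifier and delta time, flipping the MoveBack flag when it passes fixed world-space bounds either side of the origin.
; A custom event adds a signed HealthChange to Health and destroys the actor once Health reaches zero or below.
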(event EventBeginPlay)

(event Collision|EventActorBeginOverlap
  (params (OtherActor :type Actor%20Object%20Reference)))

(event EventTick
  (params (DeltaSeconds :type Float%20%28single-precision%29))
  (bind _returnvalue (Transformation|GetActorLocation))
  (bind _self self)
  (bind _speed (Variables|Default|GetSpeed))
  (bind _speed_modifier (Variables|Default|GetSpeed%20modifier))
  (bind _returnvalue_2 (Transformation|GetActorLocation _self))
  (bind _returnvalue_3 (* DeltaSeconds _speed _speed_modifier))
  (Transformation|SetActorLocation (Math|Vector|MakeVector (Math|Float|SelectFloat (- (.x _returnvalue_2) _returnvalue_3) (+ _returnvalue_3 (.x _returnvalue_2)) (Variables|Default|Getmove%20back)) (.y _returnvalue_2) (.z _returnvalue_2)) false false)
  (if (> (.x _returnvalue) 1e+03)
    (Variables|Default|Setmove%20back true)
    (elif (< (.x _returnvalue) -1e+03)
      (Variables|Default|Setmove%20back false))))

(event Custom|CustomEvent
  (params (Health%20Change :type Integer))
  (bind _output_get (Variables|Default|SetHealth (+ Health%20Change (Variables|Default|GetHealth))))
  (if (<= _output_get 0)
    (Actor|DestroyActor)))

(fn ConstructionScript)