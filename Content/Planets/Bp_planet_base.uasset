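; Base planet actor that sizes a surface component and a surrounding sphere from radius and atmosphere height values given in meters.
; The construction script uniformly scales PlanetSurface from the planet radius and sets the Sphere radius from planet radius plus atmosphere height, using fixed conversion factors.
; The event graph holds only disabled default events, so the Blueprint adds no runtime logic.
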(event EventBeginPlay)

(event Collision|EventActorBeginOverlap
  (params (OtherActor :type Actor%20Object%20Reference)))

(event EventTick
  (params (DeltaSeconds :type Float%20%28single-precision%29)))

(fn ConstructionScript
  (Transformation|SetRelativeScale3D (Variables|Default|GetPlanetSurface) (Math|Conversions|ToVector(Float) (/ (Variables|Default|Getplanet%20radius%28meters%29) 2e+01)))
  (Components|Sphere|SetSphereRadius (Variables|Default|GetSphere) (* (+ (Variables|Default|Getplanet%20radius%28meters%29) (Variables|Default|GetAtmosphere%20height%20%28meters%29)) 5e+01) true))